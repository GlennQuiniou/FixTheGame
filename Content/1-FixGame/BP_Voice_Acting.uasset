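; Interactable voice acting point that plays a 2D dialogue sound on Interact, with a six-second lock against retriggering.
; A sphere overlap with BP_CustomTPS stores the player and shows a text prompt and cube, hiding both on exit.
; While the text is visible, Tick rotates both toward the player using look-at yaw and roll with fixed pitch.
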(event OnComponentBeginOverlap(Sphere)
  (params (OverlappedComponent :type Primitive%20Component%20Object%20Reference) (OtherActor :type Actor%20Object%20Reference) (OtherComp :type Primitive%20Component%20Object%20Reference) (OtherBodyIndex :type Integer) (bFromSweep :type Boolean) (SweepResult :type Hit%20Result%20Structure%20%28by%20ref%29))
  (bind _asbp_custom_tps (Utilities|Casting|CastToBP_CustomTPS OtherActor))
  (Variables|Default|SetAs%20BP%20Custom%20TPS _asbp_custom_tps)
  (Rendering|SetVisibility (Variables|Default|GetTextRenderVoiceActing) true false)
  (Rendering|SetVisibility (Variables|Default|GetCube) true false))

(event OnComponentEndOverlap(Sphere)
  (params (OverlappedComponent :type Primitive%20Component%20Object%20Reference) (OtherActor :type Actor%20Object%20Reference) (OtherComp :type Primitive%20Component%20Object%20Reference) (OtherBodyIndex :type Integer))
  (bind _asbp_custom_tps (Utilities|Casting|CastToBP_CustomTPS OtherActor))
  (Variables|Default|SetAs%20BP%20Custom%20TPS _asbp_custom_tps)
  (Rendering|SetVisibility (Variables|Default|GetTextRenderVoiceActing) false false)
  (Rendering|SetVisibility (Variables|Default|GetCube) false false))

(event EventTick
  (params (DeltaSeconds :type Float%20%28single-precision%29))
  (bind _as_bp_custom_tps (Variables|Default|GetAs%20BP%20Custom%20TPS))
  (bind _cube (Variables|Default|GetCube))
  (bind _as_bp_custom_tps_2 (Variables|Default|GetAs%20BP%20Custom%20TPS))
  (bind _textrendervoiceacting (Variables|Default|GetTextRenderVoiceActing))
  (bind _returnvalue (Transformation|GetWorldLocation _textrendervoiceacting))
  (bind _returnvalue_2 (Transformation|GetWorldLocation _cube))
  (bind _returnvalue_3 (Transformation|GetActorLocation _as_bp_custom_tps_2))
  (bind _returnvalue_4 (Transformation|GetActorLocation _as_bp_custom_tps))
  (bind _returnvalue_5 (Math|Rotator|FindLookatRotation _returnvalue_2 _returnvalue_3))
  (bind _returnvalue_6 (Math|Rotator|FindLookatRotation _returnvalue _returnvalue_4))
  (if (Variables|/Script/Engine.SceneComponent|GetbVisible (Variables|Default|GetTextRenderVoiceActing))
    (Transformation|SetWorldRotation (Variables|Default|GetTextRenderVoiceActing) (Math|Rotator|MakeRotator (.roll _returnvalue_6) 0.0 (.yaw _returnvalue_6)) false false)
    (Transformation|SetWorldRotation (Variables|Default|GetCube) (Math|Rotator|MakeRotator (.roll _returnvalue_5) -9e+01 (.yaw _returnvalue_5)) false false)))

(event EventInteract
  (if (not (Variables|Default|GetActingEnCours))
    (Variables|Default|SetActingEnCours true)
    (Audio|PlaySound2D "/Game/1-FixGame/SonBruitage/BruitDialoge.BruitDialoge" 1.0 1.0 0.0 0 0)
    (Utilities|FlowControl|Delay 6.0)
    (Variables|Default|SetActingEnCours false)))

(fn ConstructionScript)