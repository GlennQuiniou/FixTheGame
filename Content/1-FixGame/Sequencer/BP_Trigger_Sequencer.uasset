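; One-shot trigger that plays a cinematic level sequence when the BP_CustomTPS player character overlaps it.
; At BeginPlay a box overlap query for physics bodies stores the last actor found as the sequencer actor.
; On first overlap it shows that actor's skeletal mesh, plays the sequence, then after a delay unhides a series of fire Niagara effects one after another at short intervals.
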(event Collision|EventActorBeginOverlap
  (params (OtherActor :type Actor%20Object%20Reference))
  (Utilities|Casting|CastToBP_CustomTPS OtherActor)
  (if (not (Variables|Default|GetUsageUnique))
    (Rendering|SetVisibility (Actor|GetComponentbyClass (Variables|Default|GetRefActeurSequencer) "/Script/Engine.SkeletalMeshComponent") true false)
    (Variables|Default|SetUsageUnique true)
    (bind _returnvalue (Sequencer|Player|CreateLevelSequencePlayer "/Game/1-FixGame/Sequencer/Cinematic_Level_Sequence.Cinematic_Level_Sequence"))
    (Sequencer|Player|Play _returnvalue :!class /Script/MovieScene.MovieSceneSequencePlayer)
    (Utilities|FlowControl|Delay 6.0)
    (Development|SetHiddeninGame (Variables|Default|GetNS_Fire1) false false)
    (Utilities|FlowControl|Delay 0.5)
    (Development|SetHiddeninGame (Variables|Default|GetNS_Fire2) false false)
    (Utilities|FlowControl|Delay 0.5)
    (Development|SetHiddeninGame (Variables|Default|GetNS_Fire3) false false)
    (Utilities|FlowControl|Delay 0.5)
    (Development|SetHiddeninGame (Variables|Default|GetNS_Fire4) false false)
    (Utilities|FlowControl|Delay 0.5)
    (Development|SetHiddeninGame (Variables|Default|GetNS_Fire5) false false)
    (Utilities|FlowControl|Delay 0.5)
    (Development|SetHiddeninGame (Variables|Default|GetNS_Fire6) false false)
    (Utilities|FlowControl|Delay 0.5)
    (Development|SetHiddeninGame (Variables|Default|GetNS_Fire7) false false)
    (Utilities|FlowControl|Delay 0.5)
    (Development|SetHiddeninGame (Variables|Default|GetNS_Fire8) false false)
    (Utilities|FlowControl|Delay 0.5)
    (Development|SetHiddeninGame (Variables|Default|GetNS_Fire9) false false)
    (Utilities|FlowControl|Delay 0.5)
    (Development|SetHiddeninGame (Variables|Default|GetNS_Fire10) false false)
    (Utilities|FlowControl|Delay 0.5)
    (Development|SetHiddeninGame (Variables|Default|GetNS_Fire11) false false)
    (Utilities|FlowControl|Delay 0.5)
    (Development|SetHiddeninGame (Variables|Default|GetNS_Fire12) false false)))

(event EventBeginPlay
  (bind _box (Variables|Default|GetBox))
  (bind _outactors (Collision|BoxOverlapActors (Transformation|GetWorldLocation _box) (Variables|/Script/Engine.BoxComponent|GetBoxExtent _box) (Utilities|Array|MakeArray "ObjectTypeQuery4") 0 :!class /Script/Engine.KismetSystemLibrary))
  (for _array_element _outactors
    (Variables|Default|SetRefActeurSequencer _array_element)))

(fn ConstructionScript)