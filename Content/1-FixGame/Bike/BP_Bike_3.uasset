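; BP_Bike_3 is a player-driven bike that moves by swept world offsets along its forward vector.
; Throttle and steering inputs are interpolated, and each tick yaws the bike in proportion to both while easing a speed-scaled lean into roll.
; Speed and steering feed the AB_Bike anim instance, and look inputs rotate the spring arm.
; Two hover components are initialized with the Cube at BeginPlay; leftover AddMovementInput nodes never run.
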(event EventBeginPlay
  (bind _cube (Variables|Default|GetCube))
  (bind _asab_bike (Utilities|Casting|CastToAB_Bike (Components|SkeletalMesh|GetAnimInstance (Variables|Default|GetSkeletalMeshBike))))
  (Variables|Default|SetAnimInstance _asab_bike)
  (Default|InitComponent (Variables|Default|GetHoverComponent1) _cube)
  (Default|InitComponent (Variables|Default|GetHoverComponent2) _cube))

(event EventTick
  (params (DeltaSeconds :type Float%20%28single-precision%29))
  (bind _animinstance (Variables|Default|GetAnimInstance))
  (bind _currentspeed (Variables|Default|GetCurrentSpeed))
  (Transformation|AddActorWorldOffset (* DeltaSeconds (* (Transformation|GetActorForwardVector) _currentspeed)) true)
  (Transformation|SetActorRelativeRotation (Math|Rotator|MakeRotator (Math|Interpolation|FInterpTo (Variables|Default|GetCurrentLeanAngle) (* (Variables|Default|GetCurrentSteeringAngle) (/ (Variables|Default|GetCurrentSpeed) (Variables|Default|GetMaxSpeed))) (Utilities|Time|GetWorldDeltaSeconds) 4.0) 0.0 (+ (.yaw (Transformation|GetActorRotation)) (* _currentspeed (Variables|Default|GetCurrentSteeringAngle) (Variables|Default|GetSpeedToRotationFactor) (Utilities|Time|GetWorldDeltaSeconds)))))
  (Variables|Default|SetCurrentLeanAngle (Math|Interpolation|FInterpTo (Variables|Default|GetCurrentLeanAngle) (* (Variables|Default|GetCurrentSteeringAngle) (/ (Variables|Default|GetCurrentSpeed) (Variables|Default|GetMaxSpeed))) (Utilities|Time|GetWorldDeltaSeconds) 4.0))
  (Variables|/Game/1-FixGame/Bike/AB_Bike.AB_Bike_C|SetSpeed _animinstance (Variables|Default|GetCurrentSpeed))
  (Variables|/Game/1-FixGame/Bike/AB_Bike.AB_Bike_C|SetSteering _animinstance (Variables|Default|GetCurrentSteeringAngle)))

(event Input|AxisEvents|InputAxisLookUp
  (params (AxisValue :type Float%20%28single-precision%29))
  (Transformation|AddRelativeRotation (Variables|Default|GetSpringArm) (Math|Rotator|MakeRotator 0.0 (* AxisValue -1.0) 0.0) false false))

(event Input|AxisEvents|InputAxisTurn
  (params (AxisValue :type Float%20%28single-precision%29))
  (Transformation|AddRelativeRotation (Variables|Default|GetSpringArm) (Math|Rotator|MakeRotator 0.0 0.0 AxisValue) false false))

(event Input|AxisEvents|InputAxisMoveForward
  (params (AxisValue :type Float%20%28single-precision%29))
  (Variables|Default|SetCurrentSpeed (Math|Interpolation|FInterpTo (Variables|Default|GetCurrentSpeed) (* AxisValue (Variables|Default|GetMaxSpeed)) (Utilities|Time|GetWorldDeltaSeconds) 4.0)))

(event Input|AxisEvents|InputAxisMoveRight
  (params (AxisValue :type Float%20%28single-precision%29))
  (Variables|Default|SetCurrentSteeringAngle (Math|Interpolation|FInterpTo (Variables|Default|GetCurrentSteeringAngle) (* AxisValue (Variables|Default|GetMaxSteeringAngle)) (Utilities|Time|GetWorldDeltaSeconds) 4.0)))

(event Input|KeyboardEvents|F
  (params (Key :type Key%20Structure :default "None")))

(fn ConstructionScript)