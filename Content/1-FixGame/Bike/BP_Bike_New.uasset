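; BP_Bike_New is a rideable bike pawn with interpolated throttle and steering, a spring-arm look camera and swept kinematic movement.
; Tick moves it forward, yaws and rolls it by speed and steering, and feeds both to the AB_Bike AnimInstance.
; Box overlap binds MotoRide on BP_CustomTPS, which stores the rider, possesses the bike and shows a rider mesh.
; Dismount looks unfinished: it moves the bike to Detach and possesses no pawn.
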(event OnComponentBeginOverlap(Box)
  (params (OverlappedComponent :type Primitive%20Component%20Object%20Reference) (OtherActor :type Actor%20Object%20Reference) (OtherComp :type Primitive%20Component%20Object%20Reference) (OtherBodyIndex :type Integer) (bFromSweep :type Boolean) (SweepResult :type Hit%20Result%20Structure%20%28by%20ref%29))
  (bind _asbp_custom_tps (Utilities|Casting|CastToBP_CustomTPS OtherActor))
  (EventDispatchers|BindEventtoMotoRide _asbp_custom_tps (delegate Custom|Moto%20Ride)))

(event Custom|Moto%20Ride
  (Variables|Default|SetRider (Game|GetPlayerCharacter 0))
  (Pawn|Possess (Game|GetPlayerController 0) self)
  (Rendering|SetVisibility (Variables|Default|GetSkeletalMeshCharacter) true false))

(event EventBeginPlay
  (bind _asab_bike (Utilities|Casting|CastToAB_Bike (Components|SkeletalMesh|GetAnimInstance (Variables|Character|GetMesh))))
  (Variables|Default|SetAnimInstance _asab_bike))

(event EventTick
  (params (DeltaSeconds :type Float%20%28single-precision%29))
  (bind _returnvalue (Utilities|Time|GetWorldDeltaSeconds))
  (bind _currentspeed (Variables|Default|GetCurrentSpeed))
  (bind _currentspeed_2 (Variables|Default|GetCurrentSpeed))
  (bind _maxspeed (Variables|Default|GetMaxSpeed))
  (bind _currentsteeringangle (Variables|Default|GetCurrentSteeringAngle))
  (bind _currentsteeringangle_2 (Variables|Default|GetCurrentSteeringAngle))
  (bind _animinstance (Variables|Default|GetAnimInstance))
  (bind _returnvalue_2 (/ _currentspeed_2 _maxspeed))
  (bind _returnvalue_3 (* _currentsteeringangle _returnvalue_2))
  (bind _returnvalue_4 (Math|Interpolation|FInterpTo _currentsteeringangle_2 _returnvalue_3 _returnvalue 4.0))
  (Transformation|AddActorWorldOffset (* DeltaSeconds (* (Transformation|GetActorForwardVector) _currentspeed)) true)
  (Transformation|SetActorRelativeRotation (Math|Rotator|MakeRotator _returnvalue_4 0.0 (+ (.yaw (Transformation|GetActorRotation)) (* _currentspeed (Variables|Default|GetCurrentSteeringAngle) (Variables|Default|GetSpeedToRotationFactor) (Utilities|Time|GetWorldDeltaSeconds)))))
  (Variables|Default|SetCurrentLeanAngle _returnvalue_4)
  (Variables|/Game/1-FixGame/Bike/AB_Bike.AB_Bike_C|SetSpeed _animinstance (Variables|Default|GetCurrentSpeed))
  (Variables|/Game/1-FixGame/Bike/AB_Bike.AB_Bike_C|SetSteering _animinstance (Variables|Default|GetCurrentSteeringAngle)))

(event Input|ActionEvents|InputActionMotoRide
  (params (Key :type Key%20Structure :default "None"))
  (:Pressed
    (Transformation|SetActorTransform (Transformation|GetWorldTransform (Variables|Default|GetDetach)))
    (Pawn|Possess (Game|GetPlayerController 0))))

(event Input|AxisEvents|InputAxisLookUp
  (params (AxisValue :type Float%20%28single-precision%29))
  (Transformation|AddRelativeRotation (Variables|Default|GetSpringArm) (Math|Rotator|MakeRotator 0.0 AxisValue 0.0) false false))

(event Input|AxisEvents|InputAxisTurn
  (params (AxisValue :type Float%20%28single-precision%29))
  (Transformation|AddRelativeRotation (Variables|Default|GetSpringArm) (Math|Rotator|MakeRotator 0.0 0.0 AxisValue) false false))

(event Input|AxisEvents|InputAxisMoveForward
  (params (AxisValue :type Float%20%28single-precision%29))
  (Variables|Default|SetCurrentSpeed (Math|Interpolation|FInterpTo (Variables|Default|GetCurrentSpeed) (* AxisValue (Variables|Default|GetMaxSpeed)) (Utilities|Time|GetWorldDeltaSeconds) 4.0)))

(event Input|AxisEvents|InputAxisMoveRight
  (params (AxisValue :type Float%20%28single-precision%29))
  (Variables|Default|SetCurrentSteeringAngle (Math|Interpolation|FInterpTo (Variables|Default|GetCurrentSteeringAngle) (* AxisValue (Variables|Default|GetMaxSteeringAngle)) (Utilities|Time|GetWorldDeltaSeconds) 4.0)))

(fn ConstructionScript)