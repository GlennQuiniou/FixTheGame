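; Potion pickup that adds one to the player's ScorePotion and destroys itself when its Interact event fires.
; Overlap by BP_CustomTPS stores the player reference and shows a TextRender and Cube prompt, which hides again when the overlap ends.
; While the text is visible, Tick turns both components toward the player using look-at yaw and roll with a fixed pitch.
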(event Collision|EventActorBeginOverlap
  (params (OtherActor :type Actor%20Object%20Reference))
  ;[1 1 1] Apparition et Disparition du Texte
  (bind _asbp_custom_tps (Utilities|Casting|CastToBP_CustomTPS OtherActor))
  (Variables|Default|SetRefBPCustomTPS _asbp_custom_tps)
  (Rendering|SetVisibility (Variables|Default|GetTextRenderPotion) true false)
  (Rendering|SetVisibility (Variables|Default|GetCube) true false))

(event EventInteract
  ;[1 1 1] Système d'intération, modification du nombre de potion et auto destruction
  (Variables|/Game/Blueprints/BP_CustomTPS.BP_CustomTPS_C|SetScorePotion (Variables|Default|GetRefBPCustomTPS) (+ (Variables|/Game/Blueprints/BP_CustomTPS.BP_CustomTPS_C|GetScorePotion (Variables|Default|GetRefBPCustomTPS)) 1.0))
  (Actor|DestroyActor))

(event Collision|EventActorEndOverlap
  (params (OtherActor :type Actor%20Object%20Reference))
  ;[1 1 1] Apparition et Disparition du Texte
  (bind _asbp_custom_tps (Utilities|Casting|CastToBP_CustomTPS OtherActor))
  (Variables|Default|SetRefBPCustomTPS _asbp_custom_tps)
  (Rendering|SetVisibility (Variables|Default|GetTextRenderPotion) false false)
  (Rendering|SetVisibility (Variables|Default|GetCube) false false))

(event EventTick
  (params (DeltaSeconds :type Float%20%28single-precision%29))
  (bind _refbpcustomtps (Variables|Default|GetRefBPCustomTPS))
  (bind _textrenderpotion (Variables|Default|GetTextRenderPotion))
  (bind _refbpcustomtps_2 (Variables|Default|GetRefBPCustomTPS))
  (bind _cube (Variables|Default|GetCube))
  (bind _returnvalue (Transformation|GetActorLocation _refbpcustomtps))
  (bind _returnvalue_2 (Transformation|GetWorldLocation _textrenderpotion))
  (bind _returnvalue_3 (Transformation|GetActorLocation _refbpcustomtps_2))
  (bind _returnvalue_4 (Transformation|GetWorldLocation _cube))
  (bind _returnvalue_5 (Math|Rotator|FindLookatRotation _returnvalue_4 _returnvalue))
  (bind _returnvalue_6 (Math|Rotator|FindLookatRotation _returnvalue_2 _returnvalue_3))
  ;[1 1 1] Système pour que le texte soit toujours vers le joueur
  (if (Variables|/Script/Engine.SceneComponent|GetbVisible (Variables|Default|GetTextRenderPotion))
    (Transformation|SetWorldRotation (Variables|Default|GetTextRenderPotion) (Math|Rotator|MakeRotator (.roll _returnvalue_6) 0.0 (.yaw _returnvalue_6)) false false)
    (Transformation|SetWorldRotation (Variables|Default|GetCube) (Math|Rotator|MakeRotator (.roll _returnvalue_5) -9e+01 (.yaw _returnvalue_5)) false false)))

(fn ConstructionScript)